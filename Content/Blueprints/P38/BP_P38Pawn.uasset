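; BP_P38Pawn is a player-controlled P-38 aircraft pawn that constantly moves forward and fires rockets.
; Roll and Pitch axis inputs rotate the actor locally at AngularSpeed, scaled by delta time.
; Tick spins the Left and Right meshes through RotateEvent and adds forward movement input.
; Pressing Fire spawns BP_Rocket at the Arrow's transform; the Rotation and DestroyRocket functions are defined but not called here.
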(event `InputAxis|Roll`
  (params (AxisValue :type "Float (single-precision)"))
  (`self.K2_AddActorLocalRotation` (`KismetMathLibrary.MakeRotator` (* (`self.AngularSpeed`) (`GameplayStatics.GetWorldDeltaSeconds`) AxisValue))))

(event `InputAxis|Pitch`
  (params (AxisValue :type "Float (single-precision)"))
  (`self.K2_AddActorLocalRotation` (`KismetMathLibrary.MakeRotator` 0.0 (* (`self.AngularSpeed`) (`GameplayStatics.GetWorldDeltaSeconds`) AxisValue))))

(event `self.ReceiveTick`
  (params (DeltaSeconds :type "Float (single-precision)"))
  (`self.RotateEvent` (`self.Left`))
  (`self.RotateEvent` (`self.Right`))
  (`self.AddMovementInput` (`self.GetActorForwardVector`)))

(event `RotateEvent`
  (params (Mesh :type "StaticMeshComponent Object Reference"))
  (`SceneComponent.K2_AddLocalRotation` Mesh (`KismetMathLibrary.MakeRotator` (* (`GameplayStatics.GetWorldDeltaSeconds`) (`self.RotateSpeed`))) false false))

(event `InputAction|Fire`
  (params (Key :type "Key Structure"))
  (:`Pressed`
    (`|SpawnActorFromClass` "/Game/Blueprints/BP_Rocket.BP_Rocket_C" (`SceneComponent.K2_GetComponentToWorld` (`self.Arrow`)) "Undefined" "OverrideRootScale" null null)))

(fn `DestroyRocket`
  (params (Actor :type "Actor Object Reference"))
  (`self.K2_DestroyActor` Actor))

(fn `Rotation`
  (params (StaticMesh :type "StaticMeshComponent Object Reference"))
  (`SceneComponent.K2_AddLocalRotation` StaticMesh (`KismetMathLibrary.MakeRotator` (* (`GameplayStatics.GetWorldDeltaSeconds`) (`self.RotateSpeed`))) false false))

(fn `UserConstructionScript`)